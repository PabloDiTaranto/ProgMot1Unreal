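; BP_Door is a door Blueprint that plays metal sound effects for its movement.
; PlayMovement starts the DragMetal loop-style audio only if it is not already playing.
; PlayUp and PlayDown stop the drag sound and play separate slam sounds for the two end positions.
; The events only handle audio; no movement logic is in this Blueprint.
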(event `PlayMovement`
  (bind _dragmetal (`self.DragMetal`))
  (if (not (`AudioComponent.IsPlaying` _dragmetal))
    (`AudioComponent.Play` _dragmetal 0.0)))

(event `PlayUp`
  (`AudioComponent.Stop` (`self.DragMetal`))
  (`AudioComponent.Play` (`self.MetalSlam`) 0.0))

(event `PlayDown`
  (`AudioComponent.Stop` (`self.DragMetal`))
  (`AudioComponent.Play` (`self.MetalSlam2`) 0.0))

(fn `UserConstructionScript`)