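; Player character Blueprint that handles melee combat, health, death, interaction and the HUD.
; Attack input drives a three-hit montage combo with buffered input, using notifies to trigger forward box traces that damage I_Enemy actors.
; Damage updates the health bar and plays random hit reactions; death fades in and loads DeathLevel.
; Interact input forwards press and release to the current I_Interact object.
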(event `self.ReceiveBeginPlay`
  (bind _returnvalue (`|CreateWidget` "/Game/MainCharacter/CharacterHUD.CharacterHUD_C"))
  (set `self.Hud` _returnvalue)
  (`UserWidget.AddToViewport` (`self.Hud`) 0)
  (`self.RefreshLife`))

(event `RefreshLife`
  ;[1 1 1] Refresh Life HUD
  (`/Game/MainCharacter/CharacterHUD.RefreshLifeBar` (`self.Hud`) (`self.CurrentHealth`) (`self.MaxHealth`)))

(event `InputAction|MeleeAttack`
  (params (Key :type "Key Structure"))
  (bind _mesh (`self.Mesh`))
  ;[1 1 1] Attack
  (:`Pressed`
    (if (`self.CanAttack`)
      (if (`self.canMove`)
        (if (`self.IsAttacking`)
          (set `self.SaveAttack` true)
          (else
            (set `self.IsAttacking` true)
            (switch `int` (`self.AttackCount`) :!label _label
              (:`0`
                (set `self.AttackCount` 1)
                (bind _notifyname (`|PlayMontage` _mesh "/Game/MainCharacter/Animations/PrimaryMelee_B_Slow_Montage.PrimaryMelee_B_Slow_Montage")
                  (:`OnNotifyBegin`
                    (if (== _notifyname "EffectiveAttack")
                      (`self.EffectiveAttack` 15.0)
                      (`GameplayStatics.PlaySoundAtLocation` "/Game/MainCharacter/Sounds/MainCharacter_Attack_Cue.MainCharacter_Attack_Cue" (`self.K2_GetActorLocation`) (struct) 1.0 1.0 0.0 null null null :!label _label_2)))))
              (:`1`
                (set `self.AttackCount` 2)
                (bind _notifyname_2 (`|PlayMontage` _mesh "/Game/MainCharacter/Animations/PrimaryMelee_C_Slow_Montage.PrimaryMelee_C_Slow_Montage")
                  (:`OnNotifyBegin`
                    (if (== _notifyname_2 "EffectiveAttack")
                      (`self.EffectiveAttack` 20.0)
                      (goto _label_2)))))
              (:`2`
                (set `self.AttackCount` 0)
                (bind _notifyname_3 (`|PlayMontage` _mesh "/Game/MainCharacter/Animations/PrimaryMelee_D_Slow_Montage.PrimaryMelee_D_Slow_Montage")
                  (:`OnNotifyBegin`
                    (if (== _notifyname_3 "EffectiveAttack")
                      (`self.EffectiveAttack` 25.0)
                      (goto _label_2))))))))))))

(event `ComboAttackSave`
  ;[1 1 1] Attack
  (if (`self.SaveAttack`)
    (set `self.SaveAttack` false)
    (goto _label)))

(event `ResetCombo`
  ;[1 1 1] Attack
  (set `self.AttackCount` 0)
  (set `self.SaveAttack` false)
  (set `self.IsAttacking` false))

(event `EffectiveAttack`
  (params (DamageQty :type "Float (double-precision)"))
  (bind _returnvalue (`self.K2_GetActorLocation`))
  ;[1 1 1] Attack
  (bind _outhits (`KismetSystemLibrary.BoxTraceMulti` :`Start` _returnvalue :`End` (+ _returnvalue (* (`KismetMathLibrary.GetForwardVector` (`self.K2_GetActorRotation`)) 80.0)) :`HalfSize` (40.0 40.0 80.0) :`TraceChannel` "TraceTypeQuery1" :`DrawDebugType` "ForDuration"))
  (for _array_element _outhits
    (bind (_bblockinghit _binitialoverlap _time _distance _location _impactpoint _normal _impactnormal _physmat _hitactor) (`GameplayStatics.BreakHitResult` _array_element))
    (if (`KismetSystemLibrary.DoesImplementInterface` _hitactor "/Game/Enemies/I_Enemy.I_Enemy_C")
      (message `/Game/Enemies/I_Enemy.OnDamage` _hitactor DamageQty))))

(event `DeathByFall`
  (bind _mesh (`self.Mesh`))
  ;[1 1 1] Damage
  (`SkeletalMeshComponent.SetAnimationMode` _mesh "AnimationSingleNode" :!label _label_3)
  (`SkeletalMeshComponent.PlayAnimation` _mesh "/Game/MainCharacter/Animations/Death_A.Death_A" false)
  (`GameplayStatics.PlaySoundAtLocation` "/Game/MainCharacter/Sounds/Shinbi_Effort_PainHeavy.Shinbi_Effort_PainHeavy" (`self.K2_GetActorLocation`) (struct) 1.0 1.0 0.0 null null null)
  (`self.SwapMovement` false)
  (set `self.IsDead` true)
  (bind _returnvalue (`|CreateWidget` "/Game/MainCharacter/FadeInDeath.FadeInDeath_C"))
  (`UserWidget.AddToViewport` _returnvalue 5)
  (`KismetSystemLibrary.Delay` 1.0)
  (`GameplayStatics.OpenLevel` "DeathLevel"))

(event `/Game/Global_Interfaces/IDamagable.OnDamage`
  (params (DamageIncoming :type "Float (single-precision)"))
  ;[1 1 1] Damage
  (`self.ResetCombo`)
  (if (not (`self.IsDead`))
    (set `self.CurrentHealth` (- (`self.CurrentHealth`) DamageIncoming))
    (`self.RefreshLife`)
    (if (<= (`self.CurrentHealth`) 0.0)
      (goto _label_3)
      (else
        (`self.PlayAnimMontage` (`KismetArrayLibrary.Array_Random` (`self.HitsReact`)))
        (`GameplayStatics.PlaySoundAtLocation` "/Game/MainCharacter/Sounds/MainCharacter_Damage_Cue.MainCharacter_Damage_Cue" (`self.K2_GetActorLocation`) (struct) 1.0 1.0 0.0 null null null)))))

(event `InputAction|Interactions`
  (params (Key :type "Key Structure"))
  (bind _objecttointeract (`self.ObjectToInteract`))
  (bind _caninteract (`self.CanInteract`))
  (bind _returnvalue (`KismetSystemLibrary.DoesImplementInterface` _objecttointeract "/Game/Interacts/I_Interact.I_Interact_C"))
  ;[1 1 1] Interactions
  (:`Pressed`
    (if _caninteract
      (if _returnvalue
        (message `/Game/Interacts/I_Interact.Interact` _objecttointeract))))
  (:`Released`
    (if _caninteract
      (if _returnvalue
        (message `/Game/Interacts/I_Interact.Deinteract` _objecttointeract)))))

(event `Heal`
  ;[1 1 1] Heal
  (set `self.CurrentHealth` (`self.MaxHealth`))
  (`self.RefreshLife`))

(event `InteractEnabled`
  (params (ObjectToInteract :type "Actor Object Reference"))
  ;[1 1 1] Interactions
  (set `self.ObjectToInteract` ObjectToInteract)
  (set `self.CanInteract` true))

(event `InteractDisabled`
  ;[1 1 1] Interactions
  (set `self.CanInteract` false))

(event `SwapHUD`
  ;[1 1 1] Swap HUD
  (`/Engine/EditorBlueprintResources/StandardMacros.FlipFlop`
    (:`A`
      (`Widget.SetVisibility` (`self.Hud`) "Hidden"))
    (:`B`
      (`Widget.SetVisibility` (`self.Hud`) "Visible"))))

(fn `UserConstructionScript`)