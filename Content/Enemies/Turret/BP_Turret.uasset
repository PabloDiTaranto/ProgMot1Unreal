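; Turret enemy that fires at the player while the main character is inside its trigger box, sized by Extents in the construction script.
; Entering plays MagicOrbs, turns the glass red and starts firing; leaving restores blue.
; A delay loop calls Shoot from above the actor, passing CalculateRotation's result, and repeats while PlayerInRange holds.
; ShootAvailable gates loop entry during the first cooldown.
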(event `self.ReceiveBeginPlay`
  (bind _returnvalue (`KismetMaterialLibrary.CreateDynamicMaterialInstance` "/Game/Enemies/Turret/Textures/Light_Crystal_Grounded/Glass.Glass"))
  (set `self.BlueGlassMaterial` _returnvalue)
  (bind _returnvalue_2 (`KismetMaterialLibrary.CreateDynamicMaterialInstance` "/Game/Enemies/Turret/Textures/Light_Crystal_Grounded/GlassRed.GlassRed"))
  (set `self.RedGlassMaterial` _returnvalue_2))

(event `self.Trigger.OnComponentBeginOverlap`
  (params (OverlappedComponent :type "PrimitiveComponent Object Reference") (OtherActor :type "Actor Object Reference") (OtherComp :type "PrimitiveComponent Object Reference") (OtherBodyIndex :type Integer) (bFromSweep :type Boolean) (SweepResult :type "HitResult Structure (by ref)"))
  (cast `/Game/MainCharacter/BP/BP_MainCharacter` OtherActor)
  (`AudioComponent.Play` (`self.Magic_Orbs`) 0.0)
  (set `self.PlayerInRange` true)
  (`PrimitiveComponent.SetMaterial` (`self.Glass`) 0 (`self.RedGlassMaterial`))
  (`self.ShootWhilePlayerInRange`))

(event `self.Trigger.OnComponentEndOverlap`
  (params (OverlappedComponent :type "PrimitiveComponent Object Reference") (OtherActor :type "Actor Object Reference") (OtherComp :type "PrimitiveComponent Object Reference") (OtherBodyIndex :type Integer))
  (cast `/Game/MainCharacter/BP/BP_MainCharacter` OtherActor)
  (set `self.PlayerInRange` false)
  (`PrimitiveComponent.SetMaterial` (`self.Glass`) 0 (`self.BlueGlassMaterial`)))

(event `ShootWhilePlayerInRange`
  (if (`self.ShootAvailable`)
    (set `self.ShootAvailable` false)
    (`self.Shoot` (+ (`self.K2_GetActorLocation`) (0.0 0.0 100.0)) (`KismetMathLibrary.Conv_VectorToRotator` (- (- (`self.K2_GetActorLocation` (`GameplayStatics.GetPlayerPawn` 0)) (`self.K2_GetActorLocation`)) (0.0 0.0 50.0))) :!label _label)
    (`KismetSystemLibrary.Delay` 2.0)
    (set `self.ShootAvailable` true)
    (if (`self.PlayerInRange`)
      (goto _label))))

(fn `UserConstructionScript`
  (`BoxComponent.SetBoxExtent` (`self.Trigger`) (`self.Extents`) true))