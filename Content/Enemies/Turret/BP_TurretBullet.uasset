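; BP_TurretBullet is the turret enemy's projectile, which damages the main character on overlap.
; On spawn it plays a sound, enables its sphere's collision after a short delay, and destroys itself a few seconds later.
; Any sphere overlap destroys the bullet, but only a BP_MainCharacter receives damage, through OnDamageMessage with a fixed amount.
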(event `self.ReceiveBeginPlay`
  (`GameplayStatics.PlaySoundAtLocation` "/Game/Enemies/Turret/Sounds/Lighbolt_Cue.Lighbolt_Cue" (`self.K2_GetActorLocation`) (struct) 1.0 1.0 0.0 null null null)
  (`KismetSystemLibrary.Delay` 0.2)
  (`PrimitiveComponent.SetCollisionEnabled` (`self.Sphere`) "QueryAndPhysics")
  (`KismetSystemLibrary.Delay` 5.0)
  (`self.K2_DestroyActor`))

(event `self.Sphere.OnComponentBeginOverlap`
  (params (OverlappedComponent :type "PrimitiveComponent Object Reference") (OtherActor :type "Actor Object Reference") (OtherComp :type "PrimitiveComponent Object Reference") (OtherBodyIndex :type Integer) (bFromSweep :type Boolean) (SweepResult :type "HitResult Structure (by ref)"))
  (bind _asbp_main_character (cast `/Game/MainCharacter/BP/BP_MainCharacter` OtherActor)
    (:`then`
      (message `/Game/Global_Interfaces/IDamagable.OnDamage` _asbp_main_character 3.0))
    (:`CastFailed`
      _))
  (`self.K2_DestroyActor`))

(fn `UserConstructionScript`)