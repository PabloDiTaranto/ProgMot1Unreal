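; BP_GadgetEnemy is an enemy that fires projectiles at the player and dissolves on death.
; Attack plays a montage whose GadgetAttack notify spawns a random bullet class from SpawnPoint, aimed along the actor-to-player direction.
; Non-lethal damage plays a random hit-react montage and sound.
; Death runs once: it plays an animation and sound, unpossesses, then swaps all materials to a dynamic glass instance whose Dissolve a timeline drives before destroying the actor.
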(event `self.ReceiveBeginPlay`
  ;[1 1 1] Begin Play
  (bind _returnvalue (`KismetMaterialLibrary.CreateDynamicMaterialInstance` "/Game/Enemies/M_GlassEnemies_Inst.M_GlassEnemies_Inst"))
  (set `self.MaterialInstance` _returnvalue))

(event `/Game/Enemies/I_Enemy.OnDamage`
  (params (DamageQty :type "Float (single-precision)"))
  (bind _materialinstance (`self.MaterialInstance`))
  ;[1 1 1] Damage
  (set `self.Health` (- (`self.Health`) DamageQty))
  (if (<= (`self.Health`) 0.0)
    (`/Engine/EditorBlueprintResources/StandardMacros.DoOnce` false
      (:`Completed`
        (`/Engine/EditorBlueprintResources/StandardMacros.DoOnce` false
          (:`Completed`
            (`SkeletalMeshComponent.SetAnimationMode` (`self.Mesh`) "AnimationSingleNode")
            (`SkeletalMeshComponent.PlayAnimation` (`self.Mesh`) "/Game/Enemies/GadgetEnemy/Characters/Heroes/Gadget/Animations/Death_Fwd.Death_Fwd" false)
            (`Controller.UnPossess` (`self.GetController`))
            (`GameplayStatics.PlaySoundAtLocation` "/Game/Enemies/RangeEnemyZinx/Sounds/Cue/Zinx_Death.Zinx_Death" (`self.K2_GetActorLocation`) (struct) 1.0 1.0 0.0 null null null)
            (`KismetSystemLibrary.Delay` 1.0)
            (for (_ _array_index) (`MeshComponent.GetMaterials` (`self.Mesh`))
              (`PrimitiveComponent.SetMaterial` (`self.Mesh`) _array_index _materialinstance))
            (bind (_direction _dissolve) (`Timeline|Timeline_0`)
              (:`Update`
                (`MaterialInstanceDynamic.SetScalarParameterValue` _materialinstance "Dissolve" _dissolve))
              (:`Finished`
                (`self.K2_DestroyActor`)))))))
    (else
      (`self.PlayAnimMontage` (`KismetArrayLibrary.Array_Random` (`self.HitsReacts`)))
      (`GameplayStatics.PlaySoundAtLocation` "/Game/Enemies/RangeEnemyZinx/Sounds/Cue/Zinx_Damage.Zinx_Damage" (`self.K2_GetActorLocation`) (struct) 1.0 1.0 0.0 null null null))))

(event `/Game/Enemies/I_Enemy.Attack`
  ;[1 1 1] Attack
  (bind _notifyname (`|PlayMontage` (`self.Mesh`) "/Game/Enemies/GadgetEnemy/Characters/Heroes/Gadget/Animations/Ability_Q_Montage.Ability_Q_Montage")
    (:`OnNotifyBegin`
      (if (== _notifyname "GadgetAttack")
        (`|SpawnActorFromClass` (`KismetArrayLibrary.Array_Random` (`self.Bullets`)) (`KismetMathLibrary.MakeTransform` (`SceneComponent.K2_GetComponentLocation` (`self.SpawnPoint`)) (`KismetMathLibrary.Conv_VectorToRotator` (- (`self.K2_GetActorLocation` (`GameplayStatics.GetPlayerPawn` 0)) (`self.K2_GetActorLocation`)))) "Undefined" "OverrideRootScale" self null)))))

(fn `UserConstructionScript`)