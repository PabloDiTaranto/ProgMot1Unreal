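; Khaimera boss enemy that, once initialized, shows a boss HUD and chases the player with a self-rescheduling AI move.
; A looping timer checks distance to trigger random melee montages up close or occasional ranged attacks, one slowing the player.
; Separate events toggle weapon collision for IDamagable overlap hits, launch the boss forward and spawn aimed fireballs.
; Damage randomly triggers hit reactions; death plays a material dissolve, then broadcasts BossKilled and destroys the actor.
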(event `self.ReceiveBeginPlay`
  ;[1 1 1] Begin Play
  (bind _returnvalue (`KismetMaterialLibrary.CreateDynamicMaterialInstance` "/Game/Enemies/M_GlassEnemies_Inst.M_GlassEnemies_Inst"))
  (set `self.MaterialInstance` _returnvalue))

(event `Initialize`
  ;[1 1 1] Initialize
  (`GameplayStatics.PlaySoundAtLocation` "/Game/Enemies/BossKhaimera/Sounds/Khaimera_Intro_Question_010.Khaimera_Intro_Question_010" (`self.K2_GetActorLocation`) (struct) 1.0 1.0 0.0 null null null)
  (set `self.Alive` true)
  (set `self.CurrentLife` (`self.MaxLife`))
  (`KismetSystemLibrary.Delay` 1.0)
  (`self.SeekPlayer`)
  (`self.DistancePlayer`)
  (bind _returnvalue (`|CreateWidget` "/Game/Enemies/BossKhaimera/W_BossHud.W_BossHud_C"))
  (bind _output_get (set `self.BossHud` _returnvalue))
  (`UserWidget.AddToViewport` _output_get 0)
  (`/Game/Enemies/BossKhaimera/W_BossHud.SetBoss` (`self.BossHud`) self))

(event `SeekPlayer`
  ;[1 1 1] Seek Player
  (if (`self.Alive`)
    (if (`self.IsAttacking`)
      (`MovementComponent.StopMovementImmediately` (`self.CharacterMovement`))
      (else
        (`|AIMoveTo` self (0.0 0.0 0.0) (`GameplayStatics.GetPlayerCharacter` 0) 100.0
          (:`then`
            _)
          (:`OnSuccess`
            _)
          (:`OnFail`
            _))
        (`KismetSystemLibrary.Delay` 0.2)
        (`self.SeekPlayer`)))))

(event `DistancePlayer`
  ;[1 1 1] Player Distance Func
  (`KismetSystemLibrary.K2_SetTimer` null "PlayerDistance" 1.5 true))

(event `FacePlayer`
  ;[1 1 1] Rotate To Player
  (`self.K2_SetActorRotation` (`KismetMathLibrary.FindLookAtRotation` (`self.K2_GetActorLocation`) (`self.K2_GetActorLocation` (`GameplayStatics.GetPlayerCharacter` 0)))))

(event `CloseRange`
  ;[1 1 1] Melee
  (set `self.IsAttacking` true)
  (switch `int` (`KismetMathLibrary.RandomIntegerInRange` 0 3)
    (:`0`
      (set `self.AttackMontage` "/Game/Enemies/BossKhaimera/Animations/Boss_Melee01.Boss_Melee01")
      (set `self.LaunchForce` 600.0))
    (:`1`
      (set `self.AttackMontage` "/Game/Enemies/BossKhaimera/Animations/Boss_Melee02.Boss_Melee02")
      (set `self.LaunchForce` 650.0))
    (:`2`
      (set `self.AttackMontage` "/Game/Enemies/BossKhaimera/Animations/Boss_Melee03.Boss_Melee03")
      (set `self.LaunchForce` 700.0))
    (:`3`
      (set `self.AttackMontage` "/Game/Enemies/BossKhaimera/Animations/Boss_Melee04.Boss_Melee04")
      (set `self.LaunchForce` 750.0)))
  (bind _returnvalue (`self.PlayAnimMontage` (`self.AttackMontage`) :!label _label))
  (`GameplayStatics.PlaySoundAtLocation` "/Game/Enemies/BossKhaimera/Sounds/Cues/KhaimeraAttack.KhaimeraAttack" (`self.K2_GetActorLocation`) (struct) 1.0 1.0 0.0 null null null)
  (`KismetSystemLibrary.Delay` _returnvalue)
  (set `self.IsAttacking` false)
  (`self.SeekPlayer`)
  (if (not (>= (`self.Distance`) 600.0))
    (`self.FacePlayer`)))

(event `LongRange`
  ;[1 1 1] Range
  (set `self.IsAttacking` true)
  (switch `int` (`KismetMathLibrary.RandomIntegerInRange` 0 1)
    (:`0`
      (set `self.AttackMontage` "/Game/Enemies/BossKhaimera/Animations/Boss_Range01.Boss_Range01")
      (`self.DebuffSpeed`)
      (`GameplayStatics.PlaySoundAtLocation` "/Game/Enemies/BossKhaimera/Sounds/Khaimera_SlowDebuff.Khaimera_SlowDebuff" (`self.K2_GetActorLocation`) (struct) 1.0 1.0 0.0 null null null)
      (goto _label))
    (:`1`
      (set `self.AttackMontage` "/Game/Enemies/BossKhaimera/Animations/Boss_Range02.Boss_Range02")
      (goto _label))))

(event `self.RightWeapon.OnComponentBeginOverlap`
  (params (OverlappedComponent :type "PrimitiveComponent Object Reference") (OtherActor :type "Actor Object Reference") (OtherComp :type "PrimitiveComponent Object Reference") (OtherBodyIndex :type Integer) (bFromSweep :type Boolean) (SweepResult :type "HitResult Structure (by ref)"))
  ;[1 1 1] Damage Player
  (if (`KismetSystemLibrary.DoesImplementInterface` OtherActor "/Game/Global_Interfaces/IDamagable.IDamagable_C")
    (message `/Game/Global_Interfaces/IDamagable.OnDamage` OtherActor (`self.MeleeDamage`))))

(event `self.LeftWeapon.OnComponentBeginOverlap`
  (params (OverlappedComponent :type "PrimitiveComponent Object Reference") (OtherActor :type "Actor Object Reference") (OtherComp :type "PrimitiveComponent Object Reference") (OtherBodyIndex :type Integer) (bFromSweep :type Boolean) (SweepResult :type "HitResult Structure (by ref)"))
  ;[1 1 1] Damage Player
  (if (`KismetSystemLibrary.DoesImplementInterface` OtherActor "/Game/Global_Interfaces/IDamagable.IDamagable_C")
    (message `/Game/Global_Interfaces/IDamagable.OnDamage` OtherActor (`self.MeleeDamage`))))

(event `Launcher`
  (bind _charactermovement (`self.CharacterMovement`))
  ;[1 1 1] Launch
  (set `CharacterMovementComponent.GroundFriction` 0.0 _charactermovement)
  (`self.LaunchCharacter` (+ (* (`self.GetActorForwardVector`) (`self.LaunchForce`)) (* (`self.GetActorUpVector`) (`self.Jump force`))))
  (`KismetSystemLibrary.RetriggerableDelay` 0.25)
  (set `CharacterMovementComponent.GroundFriction` 8.0 _charactermovement))

(event `/Game/Enemies/I_Enemy.OnDamage`
  (params (DamageQty :type "Float (single-precision)"))
  (bind _mesh (`self.Mesh`))
  (bind _materialinstance (`self.MaterialInstance`))
  ;[1 1 1] Damage
  (set `self.CurrentLife` (- (`self.CurrentLife`) DamageQty))
  (if (<= (`self.CurrentLife`) 0.0)
    (`/Engine/EditorBlueprintResources/StandardMacros.DoOnce` false
      (:`Completed`
        (`Widget.RemoveFromParent` (`self.BossHud`))
        (set `self.Alive` false)
        (`SkeletalMeshComponent.SetAnimationMode` _mesh "AnimationSingleNode")
        (`SkeletalMeshComponent.PlayAnimation` _mesh "/Game/Enemies/BossKhaimera/Animations/Death_B.Death_B" false)
        (`GameplayStatics.PlaySoundAtLocation` "/Game/Enemies/BossKhaimera/Sounds/Khaimera_Effort_Death_04.Khaimera_Effort_Death_04" (`self.K2_GetActorLocation`) (struct) 1.0 1.0 0.0 null null null)
        (`KismetSystemLibrary.Delay` 1.0)
        (for (_ _array_index) (`MeshComponent.GetMaterials` (`self.Mesh`))
          (`PrimitiveComponent.SetMaterial` (`self.Mesh`) _array_index _materialinstance))
        (bind (_direction _dissolve) (`Timeline|Timeline_0`)
          (:`Update`
            (`MaterialInstanceDynamic.SetScalarParameterValue` _materialinstance "Dissolve" _dissolve))
          (:`Finished`
            (`self.BossKilled`)
            (`self.K2_DestroyActor`)))))
    (else
      (`GameplayStatics.PlaySoundAtLocation` "/Game/Enemies/BossKhaimera/Sounds/Cues/KhaimeraDamaged.KhaimeraDamaged" (`self.K2_GetActorLocation`) (struct) 1.0 1.0 0.0 null null null)
      (if (>= (`KismetMathLibrary.RandomIntegerInRange` 0 10) 8)
        (`self.PlayAnimMontage` (`KismetArrayLibrary.Array_Random` (`self.HitsReacts`)))))))

(event `EnabledLeftWeaponColl`
  ;[1 1 1] Weapons Collisions
  (`PrimitiveComponent.SetCollisionEnabled` (`self.LeftWeapon`) "QueryAndPhysics"))

(event `DisabledLeftWeaponColl`
  ;[1 1 1] Weapons Collisions
  (`PrimitiveComponent.SetCollisionEnabled` (`self.LeftWeapon`) "NoCollision"))

(event `EnabledRightWeaponColl`
  ;[1 1 1] Weapons Collisions
  (`PrimitiveComponent.SetCollisionEnabled` (`self.RightWeapon`) "QueryAndPhysics"))

(event `DisableRightWeaponColl`
  ;[1 1 1] Weapons Collisions
  (`PrimitiveComponent.SetCollisionEnabled` (`self.RightWeapon`) "NoCollision"))

(event `Fireball`
  (bind _returnvalue (`SceneComponent.K2_GetComponentLocation` (`self.RightWeapon`)))
  ;[1 1 1] Fireball
  (`|SpawnActorFromClass` "/Game/Enemies/BossKhaimera/BP_BossProjectile.BP_BossProjectile_C" (`KismetMathLibrary.MakeTransform` _returnvalue (`KismetMathLibrary.FindLookAtRotation` _returnvalue (`self.K2_GetActorLocation` (`GameplayStatics.GetPlayerCharacter` 0)))) "Undefined" "OverrideRootScale" null null))

(event `DebuffSpeed`
  ;[1 1 1] DebuffSpeedToPlayer
  (bind _asbp_main_character (cast `/Game/MainCharacter/BP/BP_MainCharacter` (`GameplayStatics.GetPlayerCharacter` 0)))
  (`/Game/MainCharacter/BP/BP_MainCharacter.DebuffSpeed` _asbp_main_character))

(fn `PlayerDistance`
  ;[1 1 1] Player Distance
  (if (`self.Alive`)
    (if (not (`self.IsAttacking`))
      (bind _output_get (set `self.Distance` (`KismetMathLibrary.VSize` (- (`self.K2_GetActorLocation`) (`self.K2_GetActorLocation` (`GameplayStatics.GetPlayerCharacter` 0))))))
      ;[1 1 1] Attack Range
      (if (>= _output_get 200.0)
        (if (== (`KismetMathLibrary.RandomInteger` 4) 0)
          (`self.LongRange`)
          (else
            (`self.SeekPlayer`)))
        (else
          (`self.CloseRange`))))))

(fn `UserConstructionScript`)