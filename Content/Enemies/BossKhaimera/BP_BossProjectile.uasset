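; Fire bolt projectile for the Khaimera boss that deals fire damage to the player on hit.
; On spawn it plays a sound, enables sphere collision after a short delay and destroys itself when its lifetime ends.
; Sphere hits destroy it, except on IDamagable actors other than BP_MainCharacter, where the cast fails and it stays alive.
; Non-damagable hits also print a leftover debug string.
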(event `self.ReceiveBeginPlay`
  (`GameplayStatics.PlaySoundAtLocation` "/Game/Enemies/GadgetEnemy/Characters/Heroes/Gadget/Sounds/Soundcues/FireBoltCue.FireBoltCue" (`self.K2_GetActorLocation`) (struct) 1.0 1.0 0.0 null null null)
  (`KismetSystemLibrary.Delay` 0.2)
  (`PrimitiveComponent.SetCollisionEnabled` (`self.Sphere`) "QueryAndPhysics")
  (`KismetSystemLibrary.Delay` 10.0)
  (`self.K2_DestroyActor`))

(event `self.Sphere.OnComponentHit`
  (params (HitComponent :type "PrimitiveComponent Object Reference") (OtherActor :type "Actor Object Reference") (OtherComp :type "PrimitiveComponent Object Reference") (NormalImpulse :type "Vector Structure") (Hit :type "HitResult Structure (by ref)"))
  (if (`KismetSystemLibrary.DoesImplementInterface` OtherActor "/Game/Global_Interfaces/IDamagable.IDamagable_C")
    (bind _asbp_main_character (cast `/Game/MainCharacter/BP/BP_MainCharacter` OtherActor))
    (`/Game/MainCharacter/BP/BP_MainCharacter.DamageByFire` _asbp_main_character 30.0)
    (`self.K2_DestroyActor`)
    (else
      (`self.K2_DestroyActor`)
      (`KismetSystemLibrary.PrintString` "Hello"))))

(fn `UserConstructionScript`)