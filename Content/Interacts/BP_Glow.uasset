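; BP_Glow is a proximity highlight actor that marks its parent actor's meshes when the main character is near.
; When BP_MainCharacter begins overlapping its Box, it enables custom depth with a stencil value on every static mesh component of the parent actor, and disables custom depth on end overlap.
; Its use of GetParentActor means it works as a child actor attached to the object being highlighted.
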(event `self.Box.OnComponentBeginOverlap`
  (params (OverlappedComponent :type "PrimitiveComponent Object Reference") (OtherActor :type "Actor Object Reference") (OtherComp :type "PrimitiveComponent Object Reference") (OtherBodyIndex :type Integer) (bFromSweep :type Boolean) (SweepResult :type "HitResult Structure (by ref)"))
  (cast `/Game/MainCharacter/BP/BP_MainCharacter` OtherActor)
  (for _array_element (`self.K2_GetComponentsByClass` (`self.GetParentActor`) "/Script/Engine.StaticMeshComponent")
    (`PrimitiveComponent.SetRenderCustomDepth` _array_element true)
    (`PrimitiveComponent.SetCustomDepthStencilValue` _array_element 1)))

(event `self.Box.OnComponentEndOverlap`
  (params (OverlappedComponent :type "PrimitiveComponent Object Reference") (OtherActor :type "Actor Object Reference") (OtherComp :type "PrimitiveComponent Object Reference") (OtherBodyIndex :type Integer))
  (cast `/Game/MainCharacter/BP/BP_MainCharacter` OtherActor)
  (for _array_element (`self.K2_GetComponentsByClass` (`self.GetParentActor`) "/Script/Engine.StaticMeshComponent")
    (`PrimitiveComponent.SetRenderCustomDepth` _array_element false)
    (`PrimitiveComponent.SetCustomDepthStencilValue` _array_element 1)))

(fn `UserConstructionScript`)